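; Moving enemy that turns toward and chases the player pawn each tick while it is inside the detection zone.
; Entering the hit zone launches the player and reduces enemy health; at zero, it scatters a random number of collectables along X and destroys itself.
; Capsule hits knock the player back along the enemy's velocity and deal damage, with a cooldown made by temporarily zeroing the damage value.
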(event `self.ReceiveBeginPlay`
  ; PLAYER REF
  (bind _asbp_third_person_character (cast `/Game/PlatformersRollOut/Folder_BP/BP_ThirdPersonCharacter` (`GameplayStatics.GetPlayerPawn` 0)))
  (set `self.As BP Third Person Character` _asbp_third_person_character))

(event `self.DetectionZone.OnComponentBeginOverlap`
  (params (OverlappedComponent :type "PrimitiveComponent Object Reference") (OtherActor :type "Actor Object Reference") (OtherComp :type "PrimitiveComponent Object Reference") (OtherBodyIndex :type Integer) (bFromSweep :type Boolean) (SweepResult :type "HitResult Structure (by ref)"))
  ; PLAYER DETECTION
  (if (== OtherActor (`self.As BP Third Person Character`))
    (set `self.CanDetectPlayer` true)))

(event `LootAndDestroy`
  (bind _returnvalue (`self.GetTransform`))
  ; Loot And Destory
  (for _ (range (+ (`KismetMathLibrary.RandomIntegerInRange` 0 (`self.CoinsDropped`)) 1))
    (`|SpawnActorFromClass` "/Game/PlatformersRollOut/Folder_BP/BP_Collectable.BP_Collectable_C" (`KismetMathLibrary.MakeTransform` (`KismetMathLibrary.MakeVector` (+ (`KismetMathLibrary.RandomFloatInRange` -200.0 200.0) (.x (.location _returnvalue))) (+ (`KismetMathLibrary.RandomFloatInRange` 0.0) (.y (.location _returnvalue))) (.z (.location _returnvalue))) (.rotation _returnvalue) (.scale _returnvalue)) "Undefined" "MultiplyWithRoot" null null))
  (`self.K2_DestroyActor`))

(event `self.DetectionZone.OnComponentEndOverlap`
  (params (OverlappedComponent :type "PrimitiveComponent Object Reference") (OtherActor :type "Actor Object Reference") (OtherComp :type "PrimitiveComponent Object Reference") (OtherBodyIndex :type Integer))
  ; PLAYER DETECTION
  (if (== OtherActor (`self.As BP Third Person Character`))
    (set `self.CanDetectPlayer` false)))

(event `self.ReceiveTick`
  (params (DeltaSeconds :type "Float (single-precision)"))
  (bind (_returnvalue_x _returnvalue_y) (`KismetMathLibrary.BreakVector` (`self.K2_GetActorLocation`)))
  (bind (_returnvalue_x_2 _returnvalue_y_2) (`KismetMathLibrary.BreakVector` (`self.K2_GetActorLocation` (`self.As BP Third Person Character`))))
  ; If Player Is Detected
  (if (`self.CanDetectPlayer`)
    (`|ExecutionSequence`
      (:`then_0`
        ; Look At Player
        (`self.K2_SetActorRotation` (`KismetMathLibrary.FindLookAtRotation` (`KismetMathLibrary.MakeVector` _returnvalue_x _returnvalue_y) (`KismetMathLibrary.MakeVector` _returnvalue_x_2 _returnvalue_y_2))))
      (:`then_1`
        ; Chase Player
        (`self.AddMovementInput` (`KismetMathLibrary.Normal` (- (`self.K2_GetActorLocation` (`self.As BP Third Person Character`)) (`self.K2_GetActorLocation`))))))))

(event `self.HitZone.OnComponentBeginOverlap`
  (params (OverlappedComponent :type "PrimitiveComponent Object Reference") (OtherActor :type "Actor Object Reference") (OtherComp :type "PrimitiveComponent Object Reference") (OtherBodyIndex :type Integer) (bFromSweep :type Boolean) (SweepResult :type "HitResult Structure (by ref)"))
  ; If Player Enters Hit Zone
  (if (== OtherActor (`self.As BP Third Person Character`))
    (`|ExecutionSequence`
      (:`then_0`
        ; Launch Player
        (`self.LaunchCharacter` (`self.As BP Third Person Character`) (`self.LaunchDirection`) false false))
      (:`then_1`
        ; Calc Enemy HP
        (set `self.Health` (- (`self.Health`) (`self.EnemyDamage`)))
        ; Destroy Enemy
        (if (<= (`self.Health`) 0)
          (`self.LootAndDestroy`))))))

(event `self.CapsuleComponent.OnComponentHit`
  (params (HitComponent :type "PrimitiveComponent Object Reference") (OtherActor :type "Actor Object Reference") (OtherComp :type "PrimitiveComponent Object Reference") (NormalImpulse :type "Vector Structure") (Hit :type "HitResult Structure (by ref)"))
  ; Knockback Attack
  (if (== OtherActor (`self.As BP Third Person Character`))
    (`self.LaunchCharacter` (`self.As BP Third Person Character`) (* (`self.GetVelocity`) (`self.KnockbackStrength`)) false false)
    ; Damage Player
    (`/Game/PlatformersRollOut/Folder_BP/BP_ThirdPersonCharacter.DamagePlayer` (`self.As BP Third Person Character`) (`self.PlayerDamage`))
    ; Damage Cooldown
    (set `self.PlayerDamage` 0)
    (`KismetSystemLibrary.Delay` 1.5)
    (set `self.PlayerDamage` 1)))

(fn `UserConstructionScript`)