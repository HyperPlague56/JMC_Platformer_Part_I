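; BP_Collectable is a spinning pickup that the player collects by touching it.
; Tick applies a local rotation each frame from SpinDirection scaled by SpinSpeed, without using delta time.
; When the player pawn overlaps it, it plays the Coinrecieved sound at the placeholder mesh's location, then destroys itself after a brief delay.
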(event `self.ReceiveActorBeginOverlap`
  (params (OtherActor :type "Actor Object Reference"))
  ; Remove Obj upon player pickup
  (if (== OtherActor (`GameplayStatics.GetPlayerPawn` 0))
    (`GameplayStatics.PlaySoundAtLocation` "/Game/Audio/coin-recieved.coin-recieved" (`SceneComponent.K2_GetComponentLocation` (`self.SM_Placeholder`)) (struct) 1.0 1.0 0.0 null null null null)
    (`KismetSystemLibrary.Delay` 0.1)
    (`self.K2_DestroyActor`)))

(event `self.ReceiveTick`
  (params (DeltaSeconds :type "Float (single-precision)"))
  ; Spinning
  (`self.K2_AddActorLocalRotation` (* (`self.SpinDirection`) (`self.SpinSpeed`))))

(fn `UserConstructionScript`)