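; BP_PlatformCrumble is a platform that vanishes after the player stands on it too long, then reappears.
; A trigger zone flags the player pawn's presence, and Tick accumulates time while it is set, resetting the count otherwise.
; At the lifetime limit it hides and disables collision, waits, then restores its starting transform, visibility and collision.
; Debug prints report overlaps and the running timer.
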(event `self.ReceiveBeginPlay`
  ; SetUpVariable
  (set `self.StartTransform` (`self.GetTransform`)))

(event `self.PlatformTriggerZone.OnComponentBeginOverlap`
  (params (OverlappedComponent :type "PrimitiveComponent Object Reference") (OtherActor :type "Actor Object Reference") (OtherComp :type "PrimitiveComponent Object Reference") (OtherBodyIndex :type Integer) (bFromSweep :type Boolean) (SweepResult :type "HitResult Structure (by ref)"))
  ; ColliderCheck
  (if (== OtherActor (`GameplayStatics.GetPlayerPawn` 0))
    (`|ExecutionSequence`
      (:`then_0`
        (`KismetSystemLibrary.PrintString` "OWWW" true true (struct :`R` 0.082242 :`G` 0.060574 :`B` 0.151042 :`A` 1.0)))
      (:`then_1`
        (set `self.PlayerOnPlatform` true)))))

(event `self.PlatformTriggerZone.OnComponentEndOverlap`
  (params (OverlappedComponent :type "PrimitiveComponent Object Reference") (OtherActor :type "Actor Object Reference") (OtherComp :type "PrimitiveComponent Object Reference") (OtherBodyIndex :type Integer))
  ; ColliderCheck
  (if (== OtherActor (`GameplayStatics.GetPlayerPawn` 0))
    (`|ExecutionSequence`
      (:`then_0`
        (`KismetSystemLibrary.PrintString` "Gee Thanks Bud" true true (struct :`R` 0.082242 :`G` 0.060574 :`B` 0.151042 :`A` 1.0)))
      (:`then_1`
        (set `self.PlayerOnPlatform` false)))))

(event `self.ReceiveTick`
  (params (DeltaSeconds :type "Float (single-precision)"))
  ; SetTimerForPlatform
  (if (`self.PlayerOnPlatform`)
    (bind _output_get (set `self.TimeOnPlatform` (+ (`self.TimeOnPlatform`) DeltaSeconds)))
    (`|ExecutionSequence`
      (:`then_0`
        ; checkIfTimerIsAtLifetime
        (if (>= (`self.TimeOnPlatform`) (`self.PlatformLifetime`))
          ; HideDisableAndReappear
          (`self.SetActorHiddenInGame` true)
          (`self.SetActorEnableCollision` false)
          (`KismetSystemLibrary.Delay` (`self.TimeInvis`))
          (`self.ReturnToStart`)))
      (:`then_1`
        (`KismetSystemLibrary.PrintString` (`KismetStringLibrary.Conv_DoubleToString` _output_get))))
    (else
      (set `self.TimeOnPlatform` 0.0))))

(event `ReturnToStart`
  ; Return to default
  (`SceneComponent.K2_SetWorldTransform` (`self.DefaultSceneRoot`) (`self.StartTransform`) false false)
  (set `self.TimeOnPlatform` 0.0)
  (`self.SetActorHiddenInGame` false)
  (`self.SetActorEnableCollision` true))

(fn `UserConstructionScript`)